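; Zombie actor that takes one of four random skins on spawn, runs to a spawner-defined point, then destroys itself.
; On BeginPlay it stores its location and loops over every ZombieSpawner_BP, so the last one's MyLocation becomes the target.
; The MyZombieAnim timeline lerps the character component there without sweeping and destroys the actor when finished.
; The box overlap event is empty.
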(event `self.ReceiveBeginPlay`
  (bind _myzombiecharacter (`self.MyZombieCharacter`))
  (bind _myzombiecharacter_2 (`self.MyZombieCharacter`))
  (switch `int` (`KismetMathLibrary.RandomIntegerInRange` 0 3)
    (:`0`
      (`PrimitiveComponent.SetMaterial` _myzombiecharacter_2 0 "/Game/zombies/Materials/zombie2_Mat.zombie2_Mat"))
    (:`1`
      (`PrimitiveComponent.SetMaterial` _myzombiecharacter_2 0 "/Game/zombies/Materials/civilian_Mat.civilian_Mat"))
    (:`2`
      (`PrimitiveComponent.SetMaterial` _myzombiecharacter 0 "/Game/zombies/Materials/zombie_tank_Mat.zombie_tank_Mat"))
    (:`3`
      (`PrimitiveComponent.SetMaterial` _myzombiecharacter 0 "/Game/zombies/Materials/jumping_zombie_Mat.jumping_zombie_Mat")))
  (set `self.MyZombieLoc` (`self.K2_GetActorLocation`))
  (bind _outactors (`GameplayStatics.GetAllActorsOfClass` "/Game/zombies/ZombieSpawner_BP.ZombieSpawner_BP_C"))
  (for _array_element _outactors
    (set `self.MyPlayerLoc` (`SceneComponent.K2_GetComponentLocation` (`/Game/zombies/ZombieSpawner_BP.MyLocation` _array_element)))
    (bind (_direction _zombierun) (`Timeline|MyZombieAnim`)
      (:`Update`
        (`SceneComponent.K2_SetWorldLocation` (`self.MyZombieCharacter`) (`KismetMathLibrary.VLerp` (`self.MyZombieLoc`) (`self.MyPlayerLoc`) _zombierun) false false))
      (:`Finished`
        (`self.K2_DestroyActor`)))))

(event `self.Box.OnComponentBeginOverlap`
  (params (OverlappedComponent :type "PrimitiveComponent Object Reference") (OtherActor :type "Actor Object Reference") (OtherComp :type "PrimitiveComponent Object Reference") (OtherBodyIndex :type Integer) (bFromSweep :type Boolean) (SweepResult :type "HitResult Structure (by ref)")))

(fn `UserConstructionScript`)