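; Zombie actor that gets a random look on spawn and runs toward a target point, then destroys itself.
; BeginPlay randomly picks one of two body materials and one of two head materials.
; It reads each ZombieSpawner_BP's MyLocation as the destination, so the last one found wins.
; A timeline lerps the character component from its start location to that point without sweep, destroying the actor when finished.
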(event `self.ReceiveBeginPlay`
  (bind _myzombiehead (`self.MyZombieHead`))
  (switch `int` (`KismetMathLibrary.RandomIntegerInRange` 0 1)
    (:`0`
      (`PrimitiveComponent.SetMaterial` (`self.MyZombieCharacter`) 0 "/Game/ZombieGame/ZomBod01_Mat.ZomBod01_Mat"))
    (:`1`
      (`PrimitiveComponent.SetMaterial` (`self.MyZombieCharacter`) 0 "/Game/ZombieGame/ZomBod02_Mat.ZomBod02_Mat")))
  (switch `int` (`KismetMathLibrary.RandomIntegerInRange` 0 1)
    (:`0`
      (`PrimitiveComponent.SetMaterial` _myzombiehead 0 "/Game/ZombieGame/ZomHead01_Mat.ZomHead01_Mat"))
    (:`1`
      (`PrimitiveComponent.SetMaterial` _myzombiehead 0 "/Game/ZombieGame/ZomHead02_Mat.ZomHead02_Mat")))
  (set `self.MyZombieLoc` (`self.K2_GetActorLocation`))
  (bind _outactors (`GameplayStatics.GetAllActorsOfClass` "/Game/zombies/ZombieSpawner_BP.ZombieSpawner_BP_C"))
  (for _array_element _outactors
    (set `self.MyPlayerLoc` (`SceneComponent.K2_GetComponentLocation` (`/Game/zombies/ZombieSpawner_BP.MyLocation` _array_element)))
    (bind (_direction _zombierun) (`Timeline|MyZombieAnim`)
      (:`Update`
        (`SceneComponent.K2_SetWorldLocation` (`self.MyZombieCharacter`) (`KismetMathLibrary.VLerp` (`self.MyZombieLoc`) (`self.MyPlayerLoc`) _zombierun) false false))
      (:`Finished`
        (`self.K2_DestroyActor`)))))

(fn `UserConstructionScript`)