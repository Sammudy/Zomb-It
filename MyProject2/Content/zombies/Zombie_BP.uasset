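; Zombie actor that randomizes its look on spawn and destroys itself when a timeline finishes.
; Two random material rolls set the same slot, so the second overrides the first.
; It loops over every ZombieSpawner_BP, so the last location becomes MyPlayerLoc despite the name.
; The timeline lerps ZombieCharacter from its start toward that point, but Alpha is fixed at zero, holding it at the start.
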(event `self.ReceiveBeginPlay`
  (bind _zombiecharacter (`self.ZombieCharacter`))
  (switch `int` (`KismetMathLibrary.RandomIntegerInRange` 0 1)
    (:`0`
      (`PrimitiveComponent.SetMaterial` (`self.ZombieCharacter`) 0 "/Game/zombies/Materials/zombiemat.zombiemat"))
    (:`1`
      (`PrimitiveComponent.SetMaterial` (`self.ZombieCharacter`) 0 "/Game/ZombieGame/ZomBod01_Mat.ZomBod01_Mat")))
  (switch `int` (`KismetMathLibrary.RandomIntegerInRange` 0 1)
    (:`0`
      (`PrimitiveComponent.SetMaterial` _zombiecharacter 0 "/Game/zombies/Materials/zombiemat.zombiemat"))
    (:`1`
      (`PrimitiveComponent.SetMaterial` _zombiecharacter 0 "/Game/ZombieGame/ZomBod02_Mat.ZomBod02_Mat")))
  (set `self.MyZombieLoc` (`self.K2_GetActorLocation`))
  (bind _outactors (`GameplayStatics.GetAllActorsOfClass` "/Game/zombies/ZombieSpawner_BP.ZombieSpawner_BP_C"))
  (for _array_element _outactors
    (set `self.MyPlayerLoc` (`SceneComponent.K2_GetComponentLocation` (`Actor.RootComponent` _array_element)))
    (`Timeline|Timeline`
      (:`Update`
        (`SceneComponent.K2_SetWorldLocation` (`self.ZombieCharacter`) (`KismetMathLibrary.VLerp` (`self.MyZombieLoc`) (`self.MyPlayerLoc`)) false false))
      (:`Finished`
        (`self.K2_DestroyActor`)))))

(fn `UserConstructionScript`)