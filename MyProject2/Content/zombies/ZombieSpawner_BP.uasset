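; ZombieSpawner_BP is a spawner actor that endlessly creates Zombie_BP actors at three scene component locations.
; After a short delay on BeginPlay, a Sequence spawns one zombie at each ZombieLoc transform, ignoring collisions.
; All three spawns feed one shared Delay that loops back to the Sequence, producing a wave of three every second with no cap or stop condition.
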(event `self.ReceiveBeginPlay`
  (`KismetSystemLibrary.Delay` 1.0)
  (`|ExecutionSequence` :!label _label
    (:`then_0`
      (`|SpawnActorFromClass` "/Game/zombies/Zombie_BP.Zombie_BP_C" (`SceneComponent.K2_GetComponentToWorld` (`self.ZombieLoc01`)) "AlwaysSpawn" "MultiplyWithRoot" null null))
    (:`then_1`
      (`|SpawnActorFromClass` "/Game/zombies/Zombie_BP.Zombie_BP_C" (`SceneComponent.K2_GetComponentToWorld` (`self.ZombieLoc02`)) "AlwaysSpawn" "MultiplyWithRoot" null null))
    (:`then_2`
      (`|SpawnActorFromClass` "/Game/zombies/Zombie_BP.Zombie_BP_C" (`SceneComponent.K2_GetComponentToWorld` (`self.ZombieLoc03`)) "AlwaysSpawn" "MultiplyWithRoot" null null)))
  (`KismetSystemLibrary.Delay` 1.0)
  (goto _label))

(fn `UserConstructionScript`)